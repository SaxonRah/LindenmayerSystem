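; Demo Blueprint that sets up and grows an L-system in the construction script, apparently as a test of a branching rule set.
; LSystemComp takes a fixed axiom and two bracketed, mutually recursive rewrite rules with a configurable generation count.
; It passes render info from RenderRahSystem to TurtleComp, then runs the growth.
; BeginPlay is empty, and the spline-generation and debug-draw render calls are disconnected.
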(event `self.ReceiveBeginPlay`)

(fn `LSystem_BPTestFunction`
  (`|ExecutionSequence`
    (:`then_0`
      (`LSystemComponent.SetupLSystem` (`self.LSystemComp`) (make `LSInfo` (`self.Generations`) "1" (`|MakeArray` (make `LSRule` "1" "D-D+D+D[<+^2]-DD-D[<^-2]<^2") (make `LSRule` "2" "D+D-DD>L>>L[<+1]-DDD>L>>L>L[<-1]<1")) (`self.EmptyStringArray`))))
    (:`then_1`
      (bind _returnvalue (`LSystemComponent.RenderRahSystem` (`self.LSystemComp`)))
      (set `TurtleComponent.LSystemRenderInfo` _returnvalue (`self.TurtleComp`))
      (`LSystemComponent.GrowLSystem` (`self.LSystemComp`)))
    (:`then_2`)))

(fn `UserConstructionScript`
  (`self.LSystem_BPTestFunction`))